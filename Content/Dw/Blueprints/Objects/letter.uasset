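; A readable letter object that shows a UI prompt when something overlaps its Box.
; The overlap adds the prompt widget and enables input; pressing E swaps it for a letter image widget with mouse cursor and UI-only input.
; Both widgets receive a reference to the letter to update their text.
; Leaving the box removes the prompt and hides the cursor, but input stays enabled because DisableInput is unwired.
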(event `self.Box.OnComponentBeginOverlap`
  (params (OverlappedComponent :type "PrimitiveComponent Object Reference") (OtherActor :type "Actor Object Reference") (OtherComp :type "PrimitiveComponent Object Reference") (OtherBodyIndex :type Integer) (bFromSweep :type Boolean) (SweepResult :type "HitResult Structure (by ref)"))
  (bind _returnvalue (`|CreateWidget` "/Game/Dw/Blueprints/Objects/LetterBlueprintBtn.LetterBlueprintBtn_C"))
  (set `/Game/Dw/Blueprints/Objects/LetterBlueprintBtn.Lettermesh` self _returnvalue)
  (`/Game/Dw/Blueprints/Objects/LetterBlueprintBtn.UpdateText` _returnvalue)
  (set `self.HideLetterMessage` _returnvalue)
  (`UserWidget.AddToViewport` _returnvalue 0)
  (`self.EnableInput` (`GameplayStatics.GetPlayerController` 0)))

(event `Key|E`
  (params (Key :type "Key Structure"))
  (bind _returnvalue (`GameplayStatics.GetPlayerController` 0))
  (:`Pressed`
    (set `PlayerController.bShowMouseCursor` true _returnvalue)
    (bind _returnvalue_2 (`|CreateWidget` "/Game/Dw/Blueprints/Objects/LetterBlueprintImage.LetterBlueprintImage_C" _returnvalue))
    (set `/Game/Dw/Blueprints/Objects/LetterBlueprintImage.LetterVariableMesh` self _returnvalue_2)
    (`/Game/Dw/Blueprints/Objects/LetterBlueprintImage.UpdateLetterText` _returnvalue_2)
    (`/Game/Dw/Blueprints/Objects/LetterBlueprintImage.UpdateCloseBtnText` _returnvalue_2)
    (`Widget.RemoveFromParent` (`self.HideLetterMessage`))
    (bind _output_get (set `self.UMGLetterImage` _returnvalue_2))
    (set `/Game/Dw/Blueprints/Objects/LetterBlueprintImage.LetterVariableMesh` self _output_get)
    (`UserWidget.AddToViewport` _returnvalue_2 0)
    (`WidgetBlueprintLibrary.SetInputMode_UIOnlyEx` _returnvalue null)))

(event `self.Box.OnComponentEndOverlap`
  (params (OverlappedComponent :type "PrimitiveComponent Object Reference") (OtherActor :type "Actor Object Reference") (OtherComp :type "PrimitiveComponent Object Reference") (OtherBodyIndex :type Integer))
  (`Widget.RemoveFromParent` (`self.HideLetterMessage`))
  (set `PlayerController.bShowMouseCursor` false (`GameplayStatics.GetPlayerController` 0)))

(fn `UserConstructionScript`)