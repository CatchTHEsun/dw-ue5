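; AR_Weapon is an assault rifle weapon Blueprint that sets its magazine, reload and spread defaults in the construction script.
; Fire, gated on remaining ammo, decrements the count, plays the shoot animation and prints the count unless the player is reloading, then line traces.
; The debug-drawn Visibility trace starts at the player camera but ends at its scaled forward vector without adding the start location; hits and spread go unused.
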(event `self.Fire`
  (if (> (`self.AmmoCount`) 0)
    (`self.AmmoCheck`)
    (`self.LineTrace`)))

(fn `AmmoCheck`
  (`/Engine/EditorBlueprintResources/StandardMacros.DecrementInt` (`self.AmmoCount`)
    (:`  `
      (if (not (`/Game/Dw/Blueprints/BP_FirstPersonCharacter.IsReloading` (cast `/Game/Dw/Blueprints/BP_FirstPersonCharacter` (`GameplayStatics.GetPlayerCharacter` 0) :!pure true)))
        (`SkeletalMeshComponent.PlayAnimation` (`self.WeaponMesh`) "/Game/FPS_Assault_Pack/Animations/Rifle/A_Rifle_Shoot01.A_Rifle_Shoot01" false)
        (`KismetSystemLibrary.PrintString` (`KismetStringLibrary.Conv_IntToString` (`self.AmmoCount`)))))))

(fn `LineTrace`
  (bind _firstpersoncamera (`/Game/Dw/Blueprints/BP_FirstPersonCharacter.FirstPersonCamera` (cast `/Game/Dw/Blueprints/BP_FirstPersonCharacter` (`GameplayStatics.GetPlayerCharacter` 0) :!pure true)))
  (`KismetSystemLibrary.LineTraceSingle` :`Start` (`SceneComponent.K2_GetComponentLocation` _firstpersoncamera) :`End` (* (`SceneComponent.GetForwardVector` _firstpersoncamera) 20000.0) :`TraceChannel` "TraceTypeQuery1" :`DrawDebugType` "ForDuration"))

(fn `UserConstructionScript`
  (`parent.UserConstructionScript`)
  (set `self.MaxAmmo` 30)
  (set `self.AmmoCount` 30)
  (set `self.ReloadTime` 2.0)
  (set `self.BulletSpread` 500.0))