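; SMG weapon Blueprint that sets its magazine, reload time and spread in construction, then handles hitscan firing and timed reloading.
; Fire spends ammo, plays randomized shot audio and animation, or an empty sound when dry.
; A randomly spread camera trace finds the impact point for a bullet decal; a second muzzle trace's result is unused.
; The tracer spawn never runs because its random roll cannot reach the threshold.
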(event `self.Fire`
  (if (> (`self.AmmoCount`) 0)
    (`self.AmmoCheck`)
    (bind (_muzzlelocation _impactpoint) (`self.LineTrace`))
    (`self.SpawnDecal` _muzzlelocation _impactpoint _impactpoint)
    (else
      (`GameplayStatics.PlaySoundAtLocation` "/Game/Dw/Sound/Weapon/ar_empty.ar_empty" (`SceneComponent.K2_GetComponentLocation` (`/Game/Dw/Blueprints/BP_FirstPersonCharacter.FirstPersonCamera` (cast `/Game/Dw/Blueprints/BP_FirstPersonCharacter` (`GameplayStatics.GetPlayerCharacter` 0) :!pure true))) (struct) 1.0 1.0 0.0 null null null null))))

(event `self.Reload`
  (`SkeletalMeshComponent.PlayAnimation` (`self.WeaponMesh`) "/Game/FPS_Assault_Pack/Animations/Rifle/A_Rifle_Reload_Empty_Montage.A_Rifle_Reload_Empty_Montage" false)
  (`KismetSystemLibrary.Delay` (`self.ReloadTime`))
  (set `self.AmmoCount` (`self.MaxAmmo`))
  (`KismetSystemLibrary.PrintString` (`KismetStringLibrary.Conv_IntToString` (`self.AmmoCount`))))

(fn `AmmoCheck`
  (bind _returnvalue (`KismetMathLibrary.RandomFloatInRange` 0.7 1.2))
  (`/Engine/EditorBlueprintResources/StandardMacros.DecrementInt` (`self.AmmoCount`)
    (:`  `
      (if (not (`/Game/Dw/Blueprints/BP_FirstPersonCharacter.IsReloading` (cast `/Game/Dw/Blueprints/BP_FirstPersonCharacter` (`GameplayStatics.GetPlayerCharacter` 0) :!pure true)))
        (`GameplayStatics.PlaySoundAtLocation` "/Game/Dw/Sound/Weapon/rifle-shot.rifle-shot" (`SceneComponent.K2_GetComponentLocation` (`/Game/Dw/Blueprints/BP_FirstPersonCharacter.FirstPersonCamera` (cast `/Game/Dw/Blueprints/BP_FirstPersonCharacter` (`GameplayStatics.GetPlayerCharacter` 0) :!pure true))) (struct) (+ _returnvalue 2.5) _returnvalue 0.0 null null null null)
        (`SkeletalMeshComponent.PlayAnimation` (`self.WeaponMesh`) "/Game/FPS_Assault_Pack/Animations/Rifle/A_Rifle_Shoot01.A_Rifle_Shoot01" false)))))

(fn `LineTrace`
  (returns (MuzzleLocation :type "Vector Structure") (ImpactPoint :type "Vector Structure"))
  (bind _bulletspread (`self.BulletSpread`))
  (bind _returnvalue (`SceneComponent.K2_GetComponentLocation` (`self.Muzzle`)))
  (bind _returnvalue_2 (* _bulletspread -1.0))
  (bind _firstpersoncamera (`/Game/Dw/Blueprints/BP_FirstPersonCharacter.FirstPersonCamera` (cast `/Game/Dw/Blueprints/BP_FirstPersonCharacter` (`GameplayStatics.GetPlayerCharacter` 0) :!pure true)))
  (bind _returnvalue_3 (`SceneComponent.K2_GetComponentLocation` _firstpersoncamera))
  (bind _outhit (`KismetSystemLibrary.LineTraceSingle` _returnvalue_3 (+ (+ (* (`SceneComponent.GetForwardVector` _firstpersoncamera) 20000.0) _returnvalue_3) (`KismetMathLibrary.MakeVector` (`KismetMathLibrary.RandomFloatInRange` _returnvalue_2 _bulletspread) (`KismetMathLibrary.RandomFloatInRange` _returnvalue_2 _bulletspread) (`KismetMathLibrary.RandomFloatInRange` _returnvalue_2 _bulletspread))) "TraceTypeQuery1")) ; camera
  (bind (_bblockinghit _binitialoverlap _time _distance _location _impactpoint) (`GameplayStatics.BreakHitResult` _outhit))
  (`KismetSystemLibrary.LineTraceSingle` :`Start` _returnvalue :`End` _impactpoint :`TraceChannel` "TraceTypeQuery1" :`TraceColor` (struct :`G` 1.0 :`B` 0.215499 :`A` 1.0)) ; Gun
  (return _returnvalue _impactpoint))

(fn `SpawnDecal`
  (params (Location :type "Vector Structure") (SpawntransLocation :type "Vector Structure") (ImpactPoint :type "Vector Structure"))
  (`|SpawnActorFromClass` "/Game/Dw/Blueprints/BulletDecal_BP.BulletDecal_BP_C" (`KismetMathLibrary.MakeTransform` SpawntransLocation (`KismetMathLibrary.Conv_VectorToRotator` ImpactPoint) (0.025 0.025 0.025)) "Undefined" "OverrideRootScale" null null)
  (if (>= (`KismetMathLibrary.RandomIntegerInRange` 1 10) 150)
    (`|SpawnActorFromClass` "/Game/Dw/Blueprints/Tracer_BP.Tracer_BP_C" (`KismetMathLibrary.MakeTransform` Location (`SceneComponent.K2_GetComponentRotation` (`/Game/Dw/Blueprints/BP_FirstPersonCharacter.FirstPersonCamera` (cast `/Game/Dw/Blueprints/BP_FirstPersonCharacter` (`GameplayStatics.GetPlayerCharacter` 0) :!pure true))) (0.05 0.05 0.05)) "Undefined" "OverrideRootScale" null null))
  (return))

(fn `UserConstructionScript`
  (`parent.UserConstructionScript`)
  (set `self.MaxAmmo` 30)
  (set `self.AmmoCount` 30)
  (set `self.ReloadTime` 2.0)
  (set `self.BulletSpread` 175.0))